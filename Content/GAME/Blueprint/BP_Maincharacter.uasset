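; Player character that grapples through the level by flying to BP_HitBox targets it shoots at.
; Shoot line-traces along the camera's forward vector from the actor, stores the impact point and switches off gravity.
; Tick interpolates the actor toward just above that point with sweep, then restores half gravity once close.
; Also handles sensitivity-scaled look input gated by CanRotate and adds the UI_Info widget on BeginPlay.
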(event EventBeginPlay
  (bind _returnvalue (UserInterface|CreateWidget "/Game/GAME/Blueprint/UI_Info.UI_Info_C"))
  (UserInterface|Viewport|AddtoViewport _returnvalue 0))

(event EventTick
  (params (DeltaSeconds :type Float%20%28single-precision%29))
  (bind _returnvalue (Utilities|Time|GetWorldDeltaSeconds))
  (bind _returnvalue_2 (Transformation|GetActorLocation))
  (bind _location (Variables|Default|GetLocation))
  (bind (_x _y _z) (Math|Vector|BreakVector _location))
  (bind _returnvalue_3 (- _z -5e+01))
  (bind _returnvalue_4 (Math|Vector|MakeVector _x _y _returnvalue_3))
  (bind _returnvalue_5 (Math|Interpolation|VInterpTo _returnvalue_2 _returnvalue_4 _returnvalue 6.0))
  (if (Variables|Default|GetCanFly)
    (CallFunction|ControlGravity 0.0 false)
    (Transformation|SetActorLocation _returnvalue_5 true false)
    (if (Utilities|Operators|EqualEqual _returnvalue_5 _location 2e+02)
      (Variables|Default|SetCanFly false)
      (CallFunction|ControlGravity 0.5 true))))

(event Input|ActionEvents|InputActionShoot
  (params (Key :type Key%20Structure :default "None"))
  (bind _returnvalue (Transformation|GetActorLocation))
  (:Pressed
    (bind _outhit (Collision|LineTraceByChannel _returnvalue (+ _returnvalue (* (Math|Vector|GetForwardVector (Variables|Default|GetCamera)) 5e+03)) "TraceTypeQuery1" false 0 "None"))
    (bind _asbp_hit_box (Utilities|Casting|CastToBP_HitBox (.HitActor (Collision|BreakHitResult _outhit))))
    (CallFunction|ControlGravity 0.0 false)
    (Variables|Default|SetCanFly true)
    (Variables|Default|SetAs%20BP%20Hit%20Box _asbp_hit_box)
    (Variables|Default|SetLocation (.ImpactPoint (Collision|BreakHitResult _outhit)))))

(event Input|AxisEvents|InputAxisTurnRate
  (params (AxisValue :type Float%20%28single-precision%29))
  ;[1 0 0] Rotate
  (if (Variables|Default|GetCanRotate)
    (Pawn|Input|AddControllerPitchInput (* AxisValue (Variables|Default|GetSensi)))))

(event Input|AxisEvents|InputAxisTurnRight
  (params (AxisValue :type Float%20%28single-precision%29))
  ;[1 0 0] Rotate
  (if (Variables|Default|GetCanRotate)
    (Pawn|Input|AddControllerYawInput (* AxisValue (Variables|Default|GetSensi)))))

(fn ConstructionScript)

(fn ControlGravity
  (params (Gravity%20Scale :type Float%20%28single-precision%29) (bGravityEnabled :type Boolean))
  (Variables|/Script/Engine.CharacterMovementComponent|SetGravityScale (Variables|Character|GetCharacterMovement) Gravity%20Scale)
  (Physics|SetEnableGravity (Variables|Collision|GetCapsuleComponent) bGravityEnabled)
  (Physics|SetEnableGravity (Variables|Character|GetMesh) bGravityEnabled))